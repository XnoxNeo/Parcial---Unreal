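; Psycho is an AI enemy that hurts the third-person player on contact and can be killed through a separate hit zone.
; Overlapping its Box launches the player by JumpAdd and destroys the enemy, while overlapping its Damage component applies DamageVar damage to the player.
; Both handlers respond only to BP_ThirdPersonCharacter.
; A second, fixed-value ApplyDamage node is left unconnected, and the graph contains no movement logic.
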(event `self.Box.OnComponentBeginOverlap`
  (params (OverlappedComponent :type "PrimitiveComponent Object Reference") (OtherActor :type "Actor Object Reference") (OtherComp :type "PrimitiveComponent Object Reference") (OtherBodyIndex :type Integer) (bFromSweep :type Boolean) (SweepResult :type "HitResult Structure (by ref)"))
  ;[1 1 1] AI Death
  (bind _asbp_third_person_character (cast `/Game/ThirdPerson/Blueprints/BP_ThirdPersonCharacter` OtherActor))
  (`self.LaunchCharacter` _asbp_third_person_character (`self.JumpAdd`) false false)
  (`self.K2_DestroyActor`))

(event `self.Damage.OnComponentBeginOverlap`
  (params (OverlappedComponent :type "PrimitiveComponent Object Reference") (OtherActor :type "Actor Object Reference") (OtherComp :type "PrimitiveComponent Object Reference") (OtherBodyIndex :type Integer) (bFromSweep :type Boolean) (SweepResult :type "HitResult Structure (by ref)"))
  ;[1 1 1] Damage player on contact
  (bind _asbp_third_person_character (cast `/Game/ThirdPerson/Blueprints/BP_ThirdPersonCharacter` OtherActor))
  (`GameplayStatics.ApplyDamage` _asbp_third_person_character (`KismetMathLibrary.Conv_IntToDouble` (`self.DamageVar`))))

(fn `UserConstructionScript`)