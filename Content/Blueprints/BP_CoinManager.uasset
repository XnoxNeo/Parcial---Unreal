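; Coin manager actor that tracks coin collection in a level and handles the win screen.
; BeginPlay counts all BP_Coin actors to set and print the coin total.
; CheckCollected compares the collected count to that total, calls CompleteLevel on the game instance whether or not all are collected, then shows the win widget and mouse cursor only when they match.
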(event `self.ReceiveBeginPlay`
  (bind _outactors (`GameplayStatics.GetAllActorsOfClass` "/Game/Blueprints/BP_Coin.BP_Coin_C"))
  (set `self.MaxCoins` (`KismetArrayLibrary.Array_Length` _outactors))
  (`KismetSystemLibrary.PrintString` (`KismetStringLibrary.Conv_IntToString` (`self.MaxCoins`))))

(event `self.ReceiveTick`
  (params (DeltaSeconds :type "Float (single-precision)")))

(fn `CheckCollected`
  (bind _returnvalue (`GameplayStatics.GetPlayerController` 0))
  (set `self.AllCoinsCollected` (== (`self.CoinsCollected`) (`self.MaxCoins`)))
  (bind _asgi_game_instance (cast `/Game/Blueprints/Core/GI_GameInstance` (`GameplayStatics.GetGameInstance`)))
  (`/Game/Blueprints/Core/GI_GameInstance.CompleteLevel` _asgi_game_instance (`self.LevelToComplete`))
  (if (`self.AllCoinsCollected`)
    (bind _returnvalue_2 (`|CreateWidget` "/Game/Blueprints/BP_WinScreen.BP_WinScreen_C" _returnvalue))
    (`UserWidget.AddToViewport` _returnvalue_2 0)
    (set `PlayerController.bShowMouseCursor` true _returnvalue)))

(fn `UserConstructionScript`)