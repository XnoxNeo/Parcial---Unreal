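; BP_HealthOrb is a pickup that restores health to a BP_ThirdPersonCharacter overlapping its sphere.
; On overlap it adds AddHealth to that character, caps it through CheckMaxHealth, prints the new value, plays a sound and destroys itself.
; CheckMaxHealth looks up the character with GetActorOfClass, rather than using the overlapping one, and sets Health to a hardcoded 100 once it reaches HealthCheck.
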(event `self.Sphere.OnComponentBeginOverlap`
  (params (OverlappedComponent :type "PrimitiveComponent Object Reference") (OtherActor :type "Actor Object Reference") (OtherComp :type "PrimitiveComponent Object Reference") (OtherBodyIndex :type Integer) (bFromSweep :type Boolean) (SweepResult :type "HitResult Structure (by ref)"))
  (bind _asbp_third_person_character (cast `/Game/ThirdPerson/Blueprints/BP_ThirdPersonCharacter` OtherActor))
  (bind _output_get (set `/Game/ThirdPerson/Blueprints/BP_ThirdPersonCharacter.Health` (+ (`self.AddHealth`) (`/Game/ThirdPerson/Blueprints/BP_ThirdPersonCharacter.Health` _asbp_third_person_character)) _asbp_third_person_character))
  (`self.CheckMaxHealth`)
  (`KismetSystemLibrary.PrintString` (`KismetStringLibrary.Conv_DoubleToString` _output_get))
  (`GameplayStatics.PlaySound2D` "/Game/ThirdPerson/Blueprints/Sound/coin-recieved-230517.coin-recieved-230517" 1.0 1.0 0.0 null null)
  (`self.K2_DestroyActor`))

(fn `CheckMaxHealth`
  (bind _returnvalue (`GameplayStatics.GetActorOfClass` "/Game/ThirdPerson/Blueprints/BP_ThirdPersonCharacter.BP_ThirdPersonCharacter_C"))
  (if (>= (`/Game/ThirdPerson/Blueprints/BP_ThirdPersonCharacter.Health` _returnvalue) (`self.HealthCheck`))
    (set `/Game/ThirdPerson/Blueprints/BP_ThirdPersonCharacter.Health` 100.0 _returnvalue)))

(fn `UserConstructionScript`)