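; Door Blueprint that responds to an Interact event by rotating its DoorL component.
; A FlipFlop alternately plays and reverses Timeline, whose update applies a fixed rotation to DoorL, leaving the Lerp that reads its Door track unused.
; Tick derives DoorClosed from a separate DoorRotation timeline, which is driven only by an unreachable chain that would set DoorL's location from a rotation vector.
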(event EventBeginPlay)

(event Collision|EventActorBeginOverlap
  (params (OtherActor :type Actor%20Object%20Reference)))

(event EventTick
  (params (DeltaSeconds :type Float%20%28single-precision%29))
  (Variables|Default|SetDoorClosed (< (stale _door) 1.0)))

(event EventInteract
  (Utilities|FlowControl|FlipFlop
    (:A
      (bind _door (Timeline|Timeline Play)
        (:Update
          (Transformation|SetRelativeRotation (Variables|Default|GetDoorL) "0.000000,-100.000000,0.000000" false false))))
    (:B
      (Timeline|Timeline Reverse))))

(fn ConstructionScript)