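; BP_Bullet is a turret bullet that deals damage on contact with the player.
; When Sphere1 overlaps the third-person character, it applies fixed damage to that character's PlayerController, rather than the character, then destroys itself.
; A separate DealDamage event, not called within this graph, applies radial damage to all overlapped Pawns within AttackRange of Sphere and draws a debug sphere.
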(event `DealDamage`
  (bind _attackrange (`self.AttackRange`))
  (bind _returnvalue (`SceneComponent.K2_GetComponentLocation` (`self.Sphere`)))
  ;[1 1 1] GetDamage
  (bind _outactors (`KismetSystemLibrary.SphereOverlapActors` _returnvalue _attackrange (`|MakeArray` "ObjectTypeQuery3" :!type "EObjectTypeQuery Enum") "/Script/Engine.Actor" (`|MakeArray` self :!type "Actor Object Reference")))
  (`KismetSystemLibrary.DrawDebugSphere` _returnvalue _attackrange 12 (struct :`R` 1.0 :`A` 1.0) 5.0)
  (for _array_element _outactors
    (`GameplayStatics.ApplyDamage` _array_element (`self.Damage`) (`self.GetController`) self "/Script/Engine.DamageType")))

(event `self.Sphere1.OnComponentBeginOverlap`
  (params (OverlappedComponent :type "PrimitiveComponent Object Reference") (OtherActor :type "Actor Object Reference") (OtherComp :type "PrimitiveComponent Object Reference") (OtherBodyIndex :type Integer) (bFromSweep :type Boolean) (SweepResult :type "HitResult Structure (by ref)"))
  (bind _asbp_third_person_character (cast `/Game/ThirdPerson/Blueprints/BP_ThirdPersonCharacter` OtherActor))
  (bind _aspc_player_controller (cast `/Game/Blueprints/Core/PC_PlayerController` (`self.GetController` _asbp_third_person_character)))
  (`GameplayStatics.ApplyDamage` _aspc_player_controller 10.0 null null "/Script/Engine.DamageType")
  (`self.K2_DestroyActor`))

(fn `UserConstructionScript`)